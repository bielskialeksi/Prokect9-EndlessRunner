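; BP_RunCharacter is a runner character that handles its own death and keeps a coin count.
; Die disables input and movement, spawns an explosion effect and sound, hides the mesh, then restarts the level by console command after a short delay.
; AddCoin adds the passed amount to the Coin total.
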(event Custom|Die
  (bind _self self)
  (bind _returnvalue (Transformation|GetActorLocation _self))
  (Input|DisableInput (Game|GetPlayerController 0))
  (Pawn|Components|CharacterMovement|DisableMovement (Variables|Character|GetCharacterMovement))
  (Effects|SpawnEmitteratLocation "/Game/StarterContent/Particles/P_Explosion.P_Explosion" _returnvalue)
  (Audio|PlaySoundatLocation "/Game/StarterContent/Audio/Explosion01.Explosion01" _returnvalue "0, 0, 0" 1.0 1.0 0.0 0 0 0 0)
  (Rendering|SetVisibility (Variables|Character|GetMesh) false false)
  (Utilities|FlowControl|Delay 3.0)
  (Development|ExecuteConsoleCommand "RestartLevel" 0))

(event EventBeginPlay)

(event Collision|EventActorBeginOverlap
  (params (OtherActor :type Actor%20Object%20Reference)))

(event EventTick
  (params (DeltaSeconds :type Float%20%28single-precision%29)))

(fn ConstructionScript)

(fn AddCoin
  (params (addCoin :type Float%20%28double-precision%29))
  (Variables|Default|SetCoin (+ addCoin (Variables|Default|GetCoin))))