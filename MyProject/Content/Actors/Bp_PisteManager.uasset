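; Endless-runner manager actor that builds the track from BP_Piste tiles and restarts the level when the player dies.
; On BeginPlay it shows the CoinPrinter widget and spawns the initial tiles, each at the previous tile's attach transform.
; It binds to each tile's Exited event, with a Delete handler that spawns a new tile and destroys the old one shortly after.
; Tick polls the runner's Alive flag, triggering a delayed RestartLevel console command.
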(event Custom|Delete
  (params (NewParam :type BP%20Piste%20Object%20Reference))
  (CallFunction|CreateNextTile)
  (Utilities|FlowControl|Delay 0.5)
  (Actor|DestroyActor NewParam))

(event Custom|ChracterDie
  (bind _asbp_run_character (Utilities|Casting|CastToBP_RunCharacter (Game|Player|GetPlayerPawn 0)))
  (if (not (Variables|/Game/Actors/BP_RunCharacter.BP_RunCharacter_C|GetAlive _asbp_run_character))
    (Utilities|FlowControl|Delay 3.0)
    (Development|ExecuteConsoleCommand "RestartLevel" 0)))

(event EventBeginPlay
  (bind _returnvalue (UserInterface|CreateWidget "/Game/other/CoinPrinter.CoinPrinter_C"))
  (UserInterface|Viewport|AddtoViewport _returnvalue 0)
  (for _index (range 0 (Variables|Default|GetNumberTile))
    (CallFunction|CreateNextTile)))

(event Collision|EventActorBeginOverlap
  (params (OtherActor :type Actor%20Object%20Reference)))

(event EventTick
  (params (DeltaSeconds :type Float%20%28single-precision%29))
  (CallFunction|ChracterDie))

(fn ConstructionScript)

(fn CreateNextTile
  (bind _returnvalue (Game|SpawnActorfromClass "/Game/Actors/BP_Piste.BP_Piste_C" (Variables|Default|GetTransformLastPiste) "Undefined" "MultiplyWithRoot" 0 0))
  (bind _output_get (Variables|Default|SetTile _returnvalue))
  (bind _newparam (Default|GetAttachTransform _output_get))
  (Variables|Default|SetTransformLastPiste _newparam)
  (EventDispatchers|BindEventtoExited (Variables|Default|GetTile) (EventDispatchers|CreateEvent (Variables|Default|GetTile) :!event ExitedEvent)))