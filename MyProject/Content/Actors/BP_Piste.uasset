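; Track tile for a runner game, carrying randomized obstacles and coins, with an attach point for chaining tiles.
; The construction script rolls for one obstacle and several coins, placing them as child actors at random points inside their spawn boxes.
; The runner overlapping Exit fires the Exited dispatcher.
; Exited_Event has Bp_PisteManager create the next tile, then destroys the passed tile after a short delay.
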(event OnComponentBeginOverlap(exit)
  (params (OverlappedComponent :type Primitive%20Component%20Object%20Reference) (OtherActor :type Actor%20Object%20Reference) (OtherComp :type Primitive%20Component%20Object%20Reference) (OtherBodyIndex :type Integer) (bFromSweep :type Boolean) (SweepResult :type Hit%20Result%20Structure%20%28by%20ref%29))
  (Utilities|Casting|CastToBP_RunCharacter OtherActor)
  (Default|CallExited self))

(event Custom|Exited_Event
  (params (Tile :type BP%20Piste%20Object%20Reference))
  (bind _returnvalue (Actor|GetActorOfClass "/Game/Actors/Bp_PisteManager.Bp_PisteManager_C"))
  (Default|CreateNextTile _returnvalue)
  (Utilities|FlowControl|Delay 0.5)
  (Actor|DestroyActor Tile))

(event EventBeginPlay)

(event Collision|EventActorBeginOverlap
  (params (OtherActor :type Actor%20Object%20Reference)))

(event EventTick
  (params (DeltaSeconds :type Float%20%28single-precision%29)))

(fn ConstructionScript
  (CallFunction|SpawObstacle)
  (for _index (range 0 (Math|Float|Truncate (Variables|Default|Getmaximum%20number%20item)))
    (CallFunction|SpawnItem)))

(fn GetAttachTransform
  (return (Transformation|GetWorldTransform (Variables|Default|GetAttachPoint))))

(fn SpawObstacle
  (bind _spawnbox (Variables|Default|GetSpawnBox))
  (if (Math|Random|RandomBoolwithWeight (Variables|Default|GetObstacleSpawnChance))
    (bind _returnvalue (AddComponent|AddChildActorComponent false (Math|Transform|MakeTransform (Math|Random|RandomPointinBoundingBox (Variables|/Script/Engine.SceneComponent|GetRelativeLocation _spawnbox) (/ (Variables|/Script/Engine.BoxComponent|GetBoxExtent _spawnbox) 2.0)) "0, 0, 0" "1.000000,1.000000,1.000000")))
    (ChildActorComponent|SetChildActorClass _returnvalue (.OutItem (Utilities|Array|Random (Variables|Default|GetObstacle%20type))))))

(fn SpawnItem
  (bind _spaw_item (Variables|Default|GetSpaw%20item))
  (if (Math|Random|RandomBoolwithWeight (Variables|Default|GetPickupSpawnChance))
    (bind _returnvalue (AddComponent|AddChildActorComponent false (Math|Transform|MakeTransform (Math|Random|RandomPointinBoundingBox (Variables|/Script/Engine.SceneComponent|GetRelativeLocation _spaw_item) (/ (Variables|/Script/Engine.BoxComponent|GetBoxExtent _spaw_item) 2.0)) "0, 0, 0" "1.000000,1.000000,1.000000")))
    (ChildActorComponent|SetChildActorClass _returnvalue (Variables|Default|Getcoin))))