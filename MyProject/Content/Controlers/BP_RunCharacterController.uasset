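; BP_RunCharacterController is a controller that drives BP_RunCharacter as an auto-running character.
; On BeginPlay it casts the controlled pawn to BP_RunCharacter and stores it.
; Every Tick pushes the character along its forward vector at full scale, while the MoveRight input axis adds sideways movement along its right vector.
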(event EventBeginPlay
  (bind _asbp_run_chatacter (Utilities|Casting|CastToBP_RunCharacter (Pawn|GetControlledPawn)))
  (Variables|Default|SetRun%20Character _asbp_run_chatacter))

(event EventTick
  (params (DeltaSeconds :type Float%20%28single-precision%29))
  (bind _run_character (Variables|Default|GetRun%20Character))
  (Pawn|Input|AddMovementInput _run_character (Transformation|GetActorForwardVector _run_character) 1.0 false))

(event Input|AxisEvents|InputAxisMoveRight
  (params (AxisValue :type Float%20%28single-precision%29))
  (bind _run_character (Variables|Default|GetRun%20Character))
  (Pawn|Input|AddMovementInput _run_character (Transformation|GetActorRightVector _run_character) AxisValue false))

(fn ConstructionScript)